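; BP_Generator is an interactable generator that, when Broken, tells the player through the HUD that it needs parts.
; OnInteracted checks the Broken flag and passes the message to the HUD's MessageHandler; no repair logic is present.
; BeginPlay waits briefly, then loops over all BP_Gaz actors and copies their HUDReference, so the last one found is kept.
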(event `/Game/Blueprints/Interfaces/Int_Interaction.OnInteracted`
  (if (`self.broken`)
    (`/Game/Blueprints/PlayerHUDs/BP_PlayerHUD.Message Handler` (`self.HUD Reference`) "Generator broken, {} parts needed")))

(event `self.ReceiveBeginPlay`
  (`KismetSystemLibrary.Delay` 1.0)
  (bind _outactors (`GameplayStatics.GetAllActorsOfClass` "/Game/Blueprints/BP_Gaz.BP_Gaz_C"))
  (for _array_element _outactors
    (if true
      (set `self.HUD Reference` (`/Game/Blueprints/BP_Gaz.HUD Reference` _array_element)))))

(fn `UserConstructionScript`)