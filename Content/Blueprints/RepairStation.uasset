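; Interactable repair station that spawns a fresh BP_Kit at its Scene component's transform, keeping a single kit on the map.
; On interaction it scans for kits with an active mesh and, if KitActive is set, destroys all existing kits before spawning.
; It then passes the new kit and active state to the player's BP_Gaz through KITData.
; ToggleKITActive flips the flag when a kit is destroyed.
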(event `Toggle KIT Active`
  ;[1 1 1] Whenever KIT is destroyed this gets called
  (if (`self.kitActive`)
    (set `self.kitActive` false)
    (else
      (set `self.kitActive` true))))

(event `/Game/Blueprints/Interaction/Int_Interaction.OnInteracted`
  (bind _kitobject (`self.kitObject`))
  (bind _kitobject_2 (`self.kitObject`))
  ;[1 1 1] Since kitActive will be initialized to false, this section checks to see if there is any
  ; KIT objects active on the map
  (bind _outactors (`GameplayStatics.GetAllActorsOfClass` "/Game/Blueprints/BP_Kit.BP_Kit_C"))
  (for _array_element _outactors
    (if (`ActorComponent.IsActive` (`Character.Mesh` _array_element))
      (set `self.kitActive` true)))
  (if (`self.kitActive`)
    ;[1 1 1] This path triggers if there is an active KIT object on the map, then subsequently deletes it to spawn a new one
    (bind _outactors_2 (`GameplayStatics.GetAllActorsOfClass` "/Game/Blueprints/BP_Kit.BP_Kit_C"))
    (for _array_element_2 _outactors_2
      (`self.K2_DestroyActor` _array_element_2))
    (bind _returnvalue (`|SpawnActorFromClass` "/Game/Blueprints/BP_Kit.BP_Kit_C" (`SceneComponent.K2_GetComponentToWorld` (`self.Scene`)) "AdjustIfPossibleButAlwaysSpawn" "OverrideRootScale" null null))
    (set `self.kitObject` _returnvalue)
    (set `self.kitActive` true)
    (bind _asbp_gaz (cast `/Game/Blueprints/BP_Gaz` (`GameplayStatics.GetPlayerPawn` 0)))
    (`/Game/Blueprints/BP_Gaz.KIT Data` _asbp_gaz (`self.kitActive`) _kitobject_2 _kitobject_2)
    (else
      ;[1 1 1] This path triggers when there is no active KIT object on the map.
      (bind _returnvalue_2 (`|SpawnActorFromClass` "/Game/Blueprints/BP_Kit.BP_Kit_C" (`SceneComponent.K2_GetComponentToWorld` (`self.Scene`)) "AdjustIfPossibleButAlwaysSpawn" "OverrideRootScale" null null))
      (set `self.kitObject` _returnvalue_2)
      (set `self.kitActive` true)
      (bind _asbp_gaz_2 (cast `/Game/Blueprints/BP_Gaz` (`GameplayStatics.GetPlayerPawn` 0)))
      (`/Game/Blueprints/BP_Gaz.KIT Data` _asbp_gaz_2 (`self.kitActive`) _kitobject _kitobject))))

(fn `UserConstructionScript`)