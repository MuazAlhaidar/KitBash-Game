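; BP_GeneratorComponent is a collectible generator part actor that adds to a part count when interacted with.
; On BeginPlay, its Type selects which mesh variant to show, Part0 or Part1, while a third type has an empty branch.
; OnInteracted increments GeneratorParts on the passed GazReference, then destroys the actor.
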(event `self.ReceiveBeginPlay`
  (if (== 0 (`self.type`))
    (`SceneComponent.SetVisibility` (`self.part0`) true false)
    (elif (== 1 (`self.type`))
      (`SceneComponent.SetVisibility` (`self.part1`) true false)
      (elif (== 2 (`self.type`))
        _))))

(event `/Game/Blueprints/Interfaces/Int_Interaction.OnInteracted`
  (params (`Gaz Reference` :type "/Game/Blueprints/BP_Gaz Object Reference") (`Kit Reference` :type "/Game/Blueprints/BP_Kit Object Reference"))
  (`/Engine/EditorBlueprintResources/StandardMacros.IncrementInt` (`/Game/Blueprints/BP_Gaz.generatorParts` `Gaz Reference`)
    (:`  `
      (`self.K2_DestroyActor`))))

(fn `UserConstructionScript`)