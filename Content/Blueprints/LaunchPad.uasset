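; Launch pad that flings BP_Kit characters along world +Y and upward when they overlap it.
; The launch adds a fixed velocity to the character's current motion, independent of pad rotation.
; PadEnabled sets the Enabled flag, hides the Cylinder, calls an emitter disable with no emitter name and turns on Sphere overlap events.
; BeginPlay runs PadEnabled if Enabled is already set; the overlap handler itself never checks that flag.
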(event `self.ReceiveBeginPlay`
  (if (`self.enabled`)
    (`self.Pad Enabled`)))

(event `self.ReceiveActorBeginOverlap`
  (params (OtherActor :type "Actor Object Reference"))
  (bind _asbp_kit (cast `/Game/Blueprints/BP_Kit` OtherActor))
  (`Character.LaunchCharacter` _asbp_kit (0.0 30000.0 1200.0) false false))

(event `Pad Enabled`
  (set `self.enabled` true)
  (`SceneComponent.SetVisibility` (`self.Cylinder`) false false)
  (`FXSystemComponent.SetEmitterEnable` (`self.ParticleSystem`) "None" false)
  (set `PrimitiveComponent.bGenerateOverlapEvents` true (`self.Sphere`)))

(fn `UserConstructionScript`)