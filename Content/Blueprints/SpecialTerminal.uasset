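; Special terminal that lets Kit, when she is the player pawn, open a hacking UI tied to a launch pad.
; On interaction it saves Gaz's doors, health and disabled turrets, both characters' positions and the terminal ID to the game instance through TerminalMinigame.
; PadHacked finds the LaunchPad whose PadID matches the TerminalID, enables it and flags it in the game instance.
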(event `/Game/Blueprints/Interfaces/Int_Interaction.OnInteracted`
  (params (`Gaz Reference` :type "/Game/Blueprints/BP_Gaz Object Reference") (`Kit Reference` :type "/Game/Blueprints/BP_Kit Object Reference"))
  (set `self.Gaz Reference` `Gaz Reference`)
  (set `self.Kit Reference` `Kit Reference`)
  (if (== (`GameplayStatics.GetObjectClass` (`GameplayStatics.GetPlayerPawn` 0)) "/Game/Blueprints/BP_Kit.BP_Kit_C")
    (bind _returnvalue (`|CreateWidget` "/Game/TerminalContent/SpecialTerminalUI.SpecialTerminalUI_C"))
    (`UserWidget.AddToViewport` _returnvalue 0)
    (`self.Save Data`)))

(event `Pad Hacked`
  (`self.EnablePad`))

(fn `EnablePad`
  (bind _outactors (`GameplayStatics.GetAllActorsOfClass` "/Game/Blueprints/LaunchPad.LaunchPad_C"))
  (for _array_element _outactors
    (if (== (`/Game/Blueprints/LaunchPad.Pad ID` _array_element) (`self.terminalID`))
      (set `self.linkedPad` _array_element)
      (break)))
  (`/Game/Blueprints/LaunchPad.Pad Enabled` (`self.linkedPad`))
  (bind _asbp_game_instance (cast `/Game/Blueprints/BP_GameInstance` (`GameplayStatics.GetGameInstance`)))
  (set `/Game/Blueprints/BP_GameInstance.enabledPad` true _asbp_game_instance))

(fn `Find Disabled Turrets`
  (bind _outactors (`GameplayStatics.GetAllActorsOfClass` "/Game/Blueprints/BP_Turret.BP_Turret_C"))
  (for _array_element _outactors
    (if (`/Game/Blueprints/BP_Turret.disabled` _array_element)
      (`KismetArrayLibrary.Array_AddUnique` (`self.disabledTurrets`) (`/Game/Blueprints/BP_Turret.Turret ID` _array_element))))
  (set `/Game/Blueprints/BP_Gaz.disabledTurrets` (`self.disabledTurrets`) (`self.Gaz Reference`)))

(fn `Save Data`
  (bind _gaz_reference (`self.Gaz Reference`))
  (bind _asbp_game_instance (cast `/Game/Blueprints/BP_GameInstance` (`GameplayStatics.GetGameInstance`)))
  (`self.Find Disabled Turrets`)
  (`/Game/Blueprints/BP_GameInstance.TerminalMinigame` _asbp_game_instance (`/Game/Blueprints/BP_Gaz.DoorsUnlocked` _gaz_reference) (`/Game/Blueprints/BP_Gaz.Health` _gaz_reference) (`self.GetTransform` _gaz_reference) (`self.GetTransform` (`self.Kit Reference`)) (`self.terminalID`) (`/Game/Blueprints/BP_Gaz.disabledTurrets` _gaz_reference) 0))

(fn `UserConstructionScript`)