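; BP_GrappleHook is the grapple hook actor that travels to a target location once fired.
; Tick moves it by a swept, teleporting lerp, with an interpolation rate scaled by Speed and DistanceToTarget so shorter distances move faster.
; SendCableComponent stores a supplied cable and zeroes its end offset to center it on the hook.
; CapsuleTrace and PlayerStartedGrappleHook are stubs returning false or zero vectors.
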(event `self.ReceiveTick`
  (params (DeltaSeconds :type "Float (single-precision)"))
  (if (`self.Grapple Hook Fired`)
    (`self.K2_SetActorLocation` (`KismetMathLibrary.VLerp` (`self.K2_GetActorLocation`) (`self.Target Location`) (`KismetMathLibrary.FInterpTo` 0.0 1.0 DeltaSeconds (* (`self.Speed`) (+ 1.0 (- 1.0 (/ (`self.Distance to Target`) 2000.0)))))) true true)))

(event `/Game/Blueprints/GrappleHook/Blueprints/INT_GrappleHook.Send Cable Component`
  (params (`Used Cable Component` :type "CableComponent Object Reference"))
  ;[1 1 1] sets the cable to be at the exact center of this actor
  (bind _output_get (set `self.Cable Component` `Used Cable Component`))
  (set `CableComponent.EndLocation` (0.0 0.0 0.0) _output_get))

(fn `Capsule Trace`
  (params (`Skeletal Mesh Component` :type "SkeletalMeshComponent Object Reference") (`Player Skeletal Mesh` :type "SkeletalMeshComponent Object Reference"))
  (returns (`Hit Something ` :type Boolean))
  (return false))

(fn `Player Started Grapple Hook`
  (params (Actor :type "Actor Object Reference") (`Selected Mesh` :type "SkeletalMeshComponent Object Reference"))
  (returns (`Standing Point` :type "Vector Structure") (Angle :type "Rotator Structure"))
  (return (0.0 0.0 0.0)))

(fn `UserConstructionScript`)