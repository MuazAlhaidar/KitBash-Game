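; Grapple hook target Blueprint that checks for a clear path to the player and supplies landing data.
; CapsuleTrace picks checks by pitch toward the player: one raised capsule sweep for steep angles, otherwise a line trace plus two sweeps arcing over an elevated midpoint.
; PlayerStartedGrappleHook returns the selected mesh's location as the standing point and its look-at rotation toward the actor.
; AddTag and RemoveTag edit component tags on supplied meshes.
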(event `/Game/Blueprints/GrappleHook/Blueprints/INT_GrappleHook.Add Tag`
  (params (`Tag to Add` :type Name) (SM :type "SkeletalMeshComponent Object Reference"))
  (`KismetArrayLibrary.Array_Add` (`ActorComponent.ComponentTags` SM) `Tag to Add`))

(event `/Game/Blueprints/GrappleHook/Blueprints/INT_GrappleHook.Remove Tag`
  (params (`Tag to Remove` :type Name) (SM :type "SkeletalMeshComponent Object Reference"))
  (`KismetArrayLibrary.Array_RemoveItem` (`ActorComponent.ComponentTags` SM) `Tag to Remove`))

(fn `Capsule Trace`
  (params (`Skeletal Mesh Component` :type "SkeletalMeshComponent Object Reference") (`Player Skeletal Mesh` :type "SkeletalMeshComponent Object Reference"))
  (returns (`Hit Something ` :type Boolean))
  (locals (`SM Component` :type "SkeletalMeshComponent Object Reference") (`Player SM Component` :type "SkeletalMeshComponent Object Reference"))
  (bind _player_sm_component (`local.Player SM Component`))
  (bind _player_sm_component_2 (`local.Player SM Component`))
  (bind _player_sm_component_3 (`local.Player SM Component`))
  (bind _player_sm_component_4 (`local.Player SM Component`))
  (bind _player_sm_component_5 (`local.Player SM Component`))
  (bind _returnvalue (+ (`SceneComponent.K2_GetComponentLocation` (`local.SM Component`)) (0.0 0.0 150.0)))
  (bind _pitch (.pitch (`KismetMathLibrary.FindLookAtRotation` (`SceneComponent.K2_GetComponentLocation` (`local.SM Component`)) (`SceneComponent.K2_GetComponentLocation` (`local.Player SM Component`)))))
  (set `local.SM Component` `Skeletal Mesh Component`)
  (set `local.Player SM Component` `Player Skeletal Mesh`)
  (if (< _pitch -10.0)
    ;[1 1 1] Low Angle
    (bind (_outhit _returnvalue_2) (`KismetSystemLibrary.CapsuleTraceSingle` (+ (`SceneComponent.K2_GetComponentLocation` (`local.SM Component`)) (0.0 0.0 200.0)) (+ (`SceneComponent.K2_GetComponentLocation` _player_sm_component_5) (0.0 0.0 100.0)) 42.0 42.0 "TraceTypeQuery1" false (`|MakeArray` (`ActorComponent.GetOwner` _player_sm_component_5)) "None" false))
    (return (not _returnvalue_2))
    (elif (>= _pitch 25.0)
      ;[1 1 1] High Angle
      (bind (_outhit_2 _returnvalue_3) (`KismetSystemLibrary.CapsuleTraceSingle` (+ (`SceneComponent.K2_GetComponentLocation` (`local.SM Component`)) (0.0 0.0 300.0)) (+ (`SceneComponent.K2_GetComponentLocation` _player_sm_component_3) (0.0 0.0 100.0)) 42.0 42.0 "TraceTypeQuery1" false (`|MakeArray` (`ActorComponent.GetOwner` _player_sm_component_3)) "None" false))
      (return (not _returnvalue_3))
      (else
        (bind (_outhit_3 _returnvalue_4) (`KismetSystemLibrary.LineTraceSingle` (+ (`SceneComponent.K2_GetComponentLocation` (`local.SM Component`)) (0.0 0.0 150.0)) (+ (`SceneComponent.K2_GetComponentLocation` _player_sm_component) (0.0 0.0 100.0)) "TraceTypeQuery1" false (`|MakeArray` (`ActorComponent.GetOwner` _player_sm_component)) "None" false))
        (if _returnvalue_4
          (return false)
          (else
            (bind (_outhit_4 _returnvalue_5) (`KismetSystemLibrary.CapsuleTraceSingle` _returnvalue (+ (/ (+ _returnvalue (`SceneComponent.K2_GetComponentLocation` _player_sm_component_2)) 2) (0.0 0.0 500.0)) 42.0 42.0 "TraceTypeQuery1" false (`|MakeArray` (`ActorComponent.GetOwner` _player_sm_component_2)) "None" false))
            (if _returnvalue_5
              (return false)
              (else
                (bind (_outhit_5 _returnvalue_6) (`KismetSystemLibrary.CapsuleTraceSingle` (+ (/ (+ (+ (`SceneComponent.K2_GetComponentLocation` (`local.SM Component`)) (0.0 0.0 150.0)) (`SceneComponent.K2_GetComponentLocation` (`local.Player SM Component`))) 2) (0.0 0.0 500.0)) (+ (`SceneComponent.K2_GetComponentLocation` _player_sm_component_4) (0.0 0.0 100.0)) 42.0 42.0 "TraceTypeQuery1" false (`|MakeArray` (`ActorComponent.GetOwner` _player_sm_component_4)) "None" false))
                (return (not _returnvalue_6))))))))))

(fn `Player Started Grapple Hook`
  (params (Actor :type "Actor Object Reference") (`Selected Mesh` :type "SkeletalMeshComponent Object Reference"))
  (returns (`Standing Point` :type "Vector Structure") (Angle :type "Rotator Structure"))
  (return (`SceneComponent.K2_GetComponentLocation` `Selected Mesh`) (`KismetMathLibrary.FindLookAtRotation` (`SceneComponent.K2_GetComponentLocation` `Selected Mesh`) (`self.K2_GetActorLocation` Actor))))

(fn `UserConstructionScript`)