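; Grapple hook HUD that finds, marks and reports the point the player can hook onto.
; Each draw, it gathers "Standing Point" skeletal meshes not tagged "Hooked" from the objective actors and filters them with owner-run capsule traces and a conditions check.
; It picks the candidate nearest an offset screen center, subject to a minimum player distance.
; It draws a marker there and messages the player character, or resets it when no candidates remain.
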(event `/Game/Blueprints/GrappleHook/Blueprints/INT_GrappleHook.Send Player Skeletal Mesh`
  (params (`Player Mesh` :type "SkeletalMeshComponent Object Reference"))
  (set `self.Player Mesh` `Player Mesh`))

(event `/Game/Blueprints/GrappleHook/Blueprints/INT_GrappleHook.Set Objective`
  (params (Objective :type "Array of Actor Object Reference (by ref)"))
  (set `self.Current Objective` Objective))

(event `Check for a Mesh to Hook`
  (if (== (`KismetArrayLibrary.Array_Length` (`self.Current Objective`)) 0)
    (`/Engine/EditorBlueprintResources/StandardMacros.IsValid` (`self.Skeletal Mesh Ref`)
      (:`Is Valid`
        (if (or (`KismetArrayLibrary.Array_Contains` (`self.Looking At Meshes`) (`self.Skeletal Mesh Ref`)) (`KismetArrayLibrary.Array_Contains` (`self.Skeletal Mesh Component Array`) (`self.Skeletal Mesh Ref`)))
          (`KismetArrayLibrary.Array_Clear` (`self.Skeletal Mesh Component Array`))
          (`KismetArrayLibrary.Array_Clear` (`self.Looking At Meshes`)))))
    (else
      ;[1 1 1] check the actors for the skeletal mesh component with a "standing point" tag
      (for _array_element (`self.Current Objective`)
        (for _array_element_2 (`self.GetComponentsByTag` _array_element "/Script/Engine.SkeletalMeshComponent" "Standing Point")
          (if (`ActorComponent.ComponentHasTag` _array_element_2 "Hooked")
            ;[1 1 1] if the target with that tag is checked and its inside the array, remove it from the array
            (if (`KismetArrayLibrary.Array_Contains` (`self.Skeletal Mesh Component Array`) _array_element_2)
              (`KismetArrayLibrary.Array_RemoveItem` (`self.Skeletal Mesh Component Array`) _array_element_2)
              (`KismetArrayLibrary.Array_RemoveItem` (`self.Looking At Meshes`) _array_element_2))
            (else
              ;[1 1 1] otherwise, add it to the array
              (if (and (not (`KismetArrayLibrary.Array_Contains` (`self.Skeletal Mesh Component Array`) _array_element_2)) (`KismetArrayLibrary.Array_Contains` (`self.Current Objective`) (`ActorComponent.GetOwner` _array_element_2)))
                (if (not (`KismetArrayLibrary.Array_Contains` (`self.Skeletal Mesh Component Array`) _array_element_2))
                  (`KismetArrayLibrary.Array_Add` (`self.Skeletal Mesh Component Array`) _array_element_2)))))))
      (`self.Scan Skeletal Mesh Array`))))

(event `self.ReceiveDrawHUD`
  (params (SizeX :type Integer) (SizeY :type Integer))
  ;[1 1 1] Tick
  (`/Engine/EditorBlueprintResources/StandardMacros.IsValid` (`self.Player Mesh`)
    (:`Is Valid`
      (`self.Check for a mesh to hook`))))

(event `/Game/Blueprints/GrappleHook/Blueprints/INT_GrappleHook.Remove Element With Tag`
  (params (`Actor to Remove` :type "Actor Object Reference") (Tag :type Name))
  ;[1 1 1] Removes the element from the arrays
  (for _array_element (`self.GetComponentsByTag` `Actor to Remove` "/Script/Engine.SkeletalMeshComponent" Tag)
    (`KismetArrayLibrary.Array_RemoveItem` (`self.Skeletal Mesh Component Array`) _array_element)
    (if (`KismetArrayLibrary.Array_Contains` (`self.Looking At Meshes`) _array_element)
      (`KismetArrayLibrary.Array_RemoveItem` (`self.Looking At Meshes`) _array_element))))

(event `Scan Skeletal Mesh Array`
  (for _array_element (`self.Skeletal Mesh Component Array`)
    (bind _output_get (set `self.Skeletal Mesh Ref` _array_element))
    ;[1 1 1] make a line trace from location to player mesh, then check for the other conditions, based on that, we add it to the array or we remove it
    (bind _hit_something_ (message `/Game/Blueprints/GrappleHook/Blueprints/INT_GrappleHook.Capsule Trace` (`ActorComponent.GetOwner` _output_get) (`self.Skeletal Mesh Ref`) (`self.Player Mesh`)))
    (if (`self.Conditions Checker` _hit_something_)
      (if (not (`KismetArrayLibrary.Array_Contains` (`self.Looking At Meshes`) (`self.Skeletal Mesh Ref`)))
        (`KismetArrayLibrary.Array_Add` (`self.Looking At Meshes`) (`self.Skeletal Mesh Ref`)))
      (elif (`KismetArrayLibrary.Array_Contains` (`self.Looking At Meshes`) (`self.Skeletal Mesh Ref`))
        (`KismetArrayLibrary.Array_RemoveItem` (`self.Looking At Meshes`) (`self.Skeletal Mesh Ref`)))))
  (if (>= (`KismetArrayLibrary.Array_Length` (`self.Looking At Meshes`)) 1)
    (`self.Scan Looking at Meshes Array`)
    (else
      (message `/Game/Blueprints/GrappleHook/Blueprints/INT_GrappleHook.Reset Mesh and Actor` (`GameplayStatics.GetPlayerCharacter` 0)))))

(event `Scan Looking at Meshes Array`
  (bind (_x _y) (`KismetMathLibrary.BreakVector2D` (- (`self.Project Point` (`self.Selected Mesh`)) (20.0 20.0))))
  (for (_array_element _array_index) (`self.Looking At Meshes`)
    ;[1 1 1] Among the skeletal meshes that were selcted, get the closest to camera
    (`self.Get Closest Actor to Camera` _array_element _array_index))
  ;[1 1 1] after getting the closest, draw the material and send it to the player blueprint
  (`/Engine/EditorBlueprintResources/StandardMacros.IsValid` (`self.Selected Mesh`)
    (:`Is Valid`
      (`self.DrawMaterialSimple` "/Game/Blueprints/GrappleHook/Materials/M_HookMarker.M_HookMarker" _x _y 256.0 256.0 0.175)
      (message `/Game/Blueprints/GrappleHook/Blueprints/INT_GrappleHook.Send the Selected Mesh & Actor` (`GameplayStatics.GetPlayerCharacter` 0) (`self.Selected Mesh`) (`ActorComponent.GetOwner` (`self.Selected Mesh`))))))

(fn `Capsule Trace`
  (params (`Skeletal Mesh Component` :type "SkeletalMeshComponent Object Reference") (`Player Skeletal Mesh` :type "SkeletalMeshComponent Object Reference"))
  (returns (`Hit Something ` :type Boolean))
  (return false))

(fn `Get Closest Actor to Camera`
  (params (Target :type "SkeletalMeshComponent Object Reference") (Index :type Integer))
  (locals (`L Target` :type "SkeletalMeshComponent Object Reference"))
  (bind (_x _y) (`KismetMathLibrary.BreakVector2D` (/ (`WidgetLayoutLibrary.GetViewportSize`) 2.0)))
  (bind _returnvalue (`KismetMathLibrary.VSize2D` (- (- (`self.Project Point` (`local.L Target`)) (20.0 20.0)) (`KismetMathLibrary.MakeVector2D` (- _x (* _x 0.06)) (- _y (* _y 0.045))))))
  (set `local.L Target` Target)
  (if (== Index 0)
    (set `self.Distance from center of Screen` _returnvalue :!label _label)
    (if (>= (`KismetMathLibrary.VSize` (- (`SceneComponent.K2_GetComponentLocation` (`local.L Target`)) (`self.K2_GetActorLocation` (`GameplayStatics.GetPlayerCharacter` 0)))) (`self.Distance between Location and Character`))
      (set `self.Selected Mesh` (`local.L Target`))
      (return)
      (else
        (set `self.Selected Mesh` null)
        (return)))
    (elif (< _returnvalue (`self.Distance from center of Screen`))
      (goto _label))))

(fn `Player Started Grapple Hook`
  (params (Actor :type "Actor Object Reference") (`Selected Mesh` :type "SkeletalMeshComponent Object Reference"))
  (returns (`Standing Point` :type "Vector Structure") (Angle :type "Rotator Structure"))
  (return (0.0 0.0 0.0)))

(fn `UserConstructionScript`)