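; BP_KitOLD is an input-driven Blueprint that pushes its KIT physics component around with impulses.
; Tick caches DeltaSeconds, which the MoveForward and MoveRight axis events use to scale impulses along the fixed X and Y axes.
; The impulses are also multiplied by KIT's mass despite being applied as velocity changes, so heavier mass yields faster acceleration.
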(event `self.ReceiveTick`
  (params (DeltaSeconds :type "Float (single-precision)"))
  (set `self.Delta Seconds` DeltaSeconds))

(event `InputAxis|MoveRight`
  (params (AxisValue :type "Float (single-precision)"))
  (`PrimitiveComponent.AddImpulse` (`self.KIT`) (`KismetMathLibrary.MakeVector` 0.0 (* AxisValue (* (* (`PrimitiveComponent.GetMass` (`self.KIT`)) 10.0) (`self.Delta Seconds`)))) "None" true))

(event `InputAxis|MoveForward`
  (params (AxisValue :type "Float (single-precision)"))
  (`PrimitiveComponent.AddImpulse` (`self.KIT`) (`KismetMathLibrary.MakeVector` (* AxisValue (* (* (`PrimitiveComponent.GetMass` (`self.KIT`)) 10.0) (`self.Delta Seconds`)))) "None" true))

(fn `UserConstructionScript`)