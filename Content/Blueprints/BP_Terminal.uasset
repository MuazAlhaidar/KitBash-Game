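; BP_Terminal is a hackable terminal that unlocks doors or disables turrets when hacked.
; On interaction, if player pawn 0 is Kit, it opens TerminalUI and passes both characters' positions, Gaz's health and unlocked doors, and its TerminalID to the GameInstance's TerminalMinigame.
; Hack events search all doors or turrets for a matching ID and signal it.
; The objective-completion nodes in UnlockDoor are disconnected.
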(event `/Game/Blueprints/Interfaces/Int_Interaction.OnInteracted`
  (params (`Gaz Reference` :type "/Game/Blueprints/BP_Gaz Object Reference") (`Kit Reference` :type "/Game/Blueprints/BP_Kit Object Reference"))
  (set `self.Gaz Reference` `Gaz Reference`)
  (set `self.Kit Reference` `Kit Reference`)
  (if (== (`GameplayStatics.GetObjectClass` (`GameplayStatics.GetPlayerPawn` 0)) "/Game/Blueprints/BP_Kit.BP_Kit_C")
    (bind _returnvalue (`|CreateWidget` "/Game/TerminalContent/TerminalUI.TerminalUI_C"))
    (`UserWidget.AddToViewport` _returnvalue 0)
    (`self.Save Data`)))

(event `Door Hacked`
  (`self.UnlockDoor`))

(event `Turret Hacked`
  (`self.DisableTurret`))

(fn `DisableTurret`
  (bind _outactors (`GameplayStatics.GetAllActorsOfClass` "/Game/Blueprints/BP_Turret.BP_Turret_C"))
  (for _array_element _outactors
    (if (== (`/Game/Blueprints/BP_Turret.Turret ID` _array_element) (`self.terminalID`))
      (set `self.linkedTurret` _array_element)
      (break)))
  (`/Game/Blueprints/BP_Turret.Terminal` (`self.linkedTurret`)))

(fn `Save Data`
  (bind _gaz_reference (`self.Gaz Reference`))
  (bind _asbp_game_instance (cast `/Game/Blueprints/BP_GameInstance` (`GameplayStatics.GetGameInstance`)))
  (`/Game/Blueprints/BP_GameInstance.TerminalMinigame` _asbp_game_instance (`/Game/Blueprints/BP_Gaz.DoorsUnlocked` _gaz_reference) (`/Game/Blueprints/BP_Gaz.Health` _gaz_reference) (`self.GetTransform` _gaz_reference) (`self.GetTransform` (`self.Kit Reference`)) (`self.terminalID`)))

(fn `UnlockDoor`
  (bind _outactors (`GameplayStatics.GetAllActorsOfClass` "/Game/Blueprints/BP_Door.BP_Door_C"))
  (for _array_element _outactors
    (if (== (`/Game/Blueprints/BP_Door.doorID` _array_element) (`self.terminalID`))
      (set `self.linkedDoor` _array_element)
      (break)))
  (`/Game/Blueprints/BP_Door.TerminalSignal` (`self.linkedDoor`))
  (`KismetSystemLibrary.PrintString` (`KismetStringLibrary.Concat_StrStr` "Terminal sending command to door, ID: " (`KismetStringLibrary.Conv_IntToString` (`self.terminalID`)))))

(fn `UserConstructionScript`)