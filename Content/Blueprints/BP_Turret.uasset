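; BP_Turret is a turret that aims and fires at BP_Gaz pawns it spots through PawnSensing.
; On each sighting it snaps its actor rotation to face the target, then spawns a BP_Projectile at the ProjectileSpawn transform and launches it with a forward impulse scaled by ShootForce.
; A SpawnProjectile flag, reset after a short delay, throttles the fire rate.
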(event `self.PawnSensing.OnSeePawn`
  (params (Pawn :type "Pawn Object Reference"))
  (bind (_returnvalue_location _returnvalue_rotation) (`KismetMathLibrary.BreakTransform` (`SceneComponent.K2_GetComponentToWorld` (`self.ProjectileSpawn`))))
  (bind _asbp_gaz (cast `/Game/Blueprints/BP_Gaz` Pawn))
  (`|ExecutionSequence`
    (:`then_0`
      (`self.K2_SetActorRotation` (`KismetMathLibrary.FindLookAtRotation` (`self.K2_GetActorLocation`) (`self.K2_GetActorLocation` _asbp_gaz))))
    (:`then_1`
      (if (`self.spawnProjectile`)
        (bind _returnvalue (`|SpawnActorFromClass` "/Game/Blueprints/BP_Projectile.BP_Projectile_C" (`KismetMathLibrary.MakeTransform` _returnvalue_location _returnvalue_rotation) "AdjustIfPossibleButAlwaysSpawn" "OverrideRootScale" null null))
        (bind _sphere1 (`/Game/Blueprints/BP_Projectile.Sphere1` _returnvalue))
        (`PrimitiveComponent.AddImpulse` _sphere1 (* (`SceneComponent.GetForwardVector` _sphere1) (`self.Shoot Force`)) "None" true)
        (set `self.spawnProjectile` false)
        (`KismetSystemLibrary.Delay` 0.2)
        (set `self.spawnProjectile` true)))))

(fn `UserConstructionScript`)