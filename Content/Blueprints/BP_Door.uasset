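; BP_Door is a lockable sliding door that a terminal signal unlocks and the player's BP_Gaz pawn opens or closes.
; Unlocking reveals two sphere components and enables overlap events on the collision box.
; Interaction toggles a timeline forward or in reverse, moving the door along Z with sweep.
; When the timeline finishes, the door reports ObjectiveComplete to the stored Gaz reference.
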(event `TerminalSignal`
  (`KismetSystemLibrary.PrintString` "door received unlock command")
  (`self.UnlockDoor`))

(event `/Game/Blueprints/Interfaces/Int_Interaction.OnInteracted`
  (params (`Gaz Reference` :type "/Game/Blueprints/BP_Gaz Object Reference") (`Kit Reference` :type "/Game/Blueprints/BP_Kit Object Reference"))
  (bind (_closedlocation_x _closedlocation_y) (`KismetMathLibrary.BreakVector` (`self.closedLocation`)))
  (set `self.Gaz Reference` `Gaz Reference`)
  (if (and (`self.isUnlocked`) (== (`GameplayStatics.GetObjectClass` (`GameplayStatics.GetPlayerPawn` 0)) "/Game/Blueprints/BP_Gaz.BP_Gaz_C"))
    (if (`self.isOpen`)
      (set `self.isOpen` false)
      (bind (_direction _doortrack) (`Timeline|Timeline_0` :!via `Reverse` :!label _label)
        (:`Update`
          (`SceneComponent.K2_SetRelativeLocation` (`self.Door`) (`KismetMathLibrary.MakeVector` _closedlocation_x _closedlocation_y (* _doortrack 388.0)) true false))
        (:`Finished`
          (`/Game/Blueprints/BP_Gaz.Objective Complete` (`self.Gaz Reference`))))
      (else
        (set `self.isOpen` true)
        (goto _label)))))

(event `self.ReceiveBeginPlay`
  (set `self.closedLocation` (`SceneComponent.RelativeLocation` (`self.Door`)))
  (set `self.isOpen` false)
  (if (not (`self.isUnlocked`))
    (`SceneComponent.SetVisibility` (`self.Sphere`) false false)
    (`SceneComponent.SetVisibility` (`self.Sphere1`) false false)))

(fn `UnlockDoor`
  (set `self.isUnlocked` true)
  (`SceneComponent.SetVisibility` (`self.Sphere`) true false)
  (`SceneComponent.SetVisibility` (`self.Sphere1`) true false)
  (set `PrimitiveComponent.bGenerateOverlapEvents` true (`self.CollisionBox`)))

(fn `UserConstructionScript`)