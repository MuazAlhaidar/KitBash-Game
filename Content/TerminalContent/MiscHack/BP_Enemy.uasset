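; Moving enemy for the hack minigame that fails the hack when the player touches it.
; The construction script feeds StartLoc, EndLoc and Duration into InterpToMovement as a two-point relative path.
; When CollisionBox overlaps an actor of exactly BP_Player class, the enemy destroys itself, shows the HackFailed widget, switches to UI-only input with a cursor and pauses the game.
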(event `self.Collision Box.OnComponentBeginOverlap`
  (params (OverlappedComponent :type "PrimitiveComponent Object Reference") (OtherActor :type "Actor Object Reference") (OtherComp :type "PrimitiveComponent Object Reference") (OtherBodyIndex :type Integer) (bFromSweep :type Boolean) (SweepResult :type "HitResult Structure (by ref)"))
  (bind _returnvalue (`GameplayStatics.GetPlayerController` 0))
  ;[1 1 1] Kill the player
  (if (== "/Game/TerminalContent/MiscHack/BP_Player.BP_Player_C" (`GameplayStatics.GetObjectClass` OtherActor))
    (`self.K2_DestroyActor`)
    (bind _returnvalue_2 (`|CreateWidget` "/Game/TerminalContent/HackFailed.HackFailed_C" _returnvalue))
    (`UserWidget.AddToViewport` _returnvalue_2 0)
    (`WidgetBlueprintLibrary.SetInputMode_UIOnlyEx` _returnvalue null)
    (set `PlayerController.bShowMouseCursor` true _returnvalue)
    (`GameplayStatics.SetGamePaused` true)))

(fn `UserConstructionScript`
  (bind _interptomovement (`self.InterpToMovement`))
  (set `InterpToMovementComponent.ControlPoints` (`|MakeArray` (make `InterpControlPoint` (`self.Start_Loc`)) (make `InterpControlPoint` (`self.End_Loc`))) _interptomovement)
  (set `InterpToMovementComponent.Duration` (`self.Duration`) _interptomovement))